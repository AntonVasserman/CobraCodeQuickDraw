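; BP_SamuraiPawn is a samurai pawn for QuickDraw that slides its Paper2D sprite in when play begins.
; BeginPlay caches the world locations of the sprite and a destination marker, sets the timeline's play rate, then triggers SlideIn.
; The SlideInAnim timeline lerps between those two points, applying the world-space values as the sprite's relative location without sweeping.
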(event Custom|SlideIn
  (bind _alpha (Timeline|SlideInAnim Play)
    (:Update
      (Transformation|SetRelativeLocation (Variables|Default|GetPaperSpriteComp) (Math|Vector|Lerp(Vector) (Variables|Default|GetSlideInStartLocation) (Variables|Default|GetSlideInDestinationLocation) _alpha) false false))))

(event EventBeginPlay
  (Variables|Default|SetSlideInStartLocation (Transformation|GetWorldLocation (Variables|Default|GetPaperSpriteComp)))
  (Variables|Default|SetSlideInDestinationLocation (Transformation|GetWorldLocation (Variables|Default|GetSlideInDestinationMark)))
  (Components|Timeline|SetPlayRate (Variables|Default|GetSlideInAnim) (Variables|Default|GetSlideInPlayRate))
  (CallFunction|Slidein))

(fn ConstructionScript)